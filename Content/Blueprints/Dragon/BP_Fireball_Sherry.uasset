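; BP_Fireball_Sherry is a dragon fireball projectile, launched at a local-space initial velocity.
; Overlaps and hits route to a server event that ignores BP_RunnableDragon and BP_Fireball actors.
; Damageable targets take direct damage and trigger radial splash around the fireball.
; Every accepted impact multicasts explosion effects and sound, destroys the fireball and spawns a stationary BP_Firebreath near the impact from within the multicast.
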(event `/Game/Blueprints/Dragon/BP_Fireball.ReceiveBeginPlay`
  (`ProjectileMovementComponent.SetVelocityInLocalSpace` (`self.ProjectileMovement`) (`self.InitialVel`)))

(event `self.ReceiveTick`
  (params (DeltaSeconds :type "Float (single-precision)")))

(event `self.ReceiveActorBeginOverlap`
  (params (OtherActor :type "Actor Object Reference"))
  (`self.ServerFireballHit` OtherActor (`SceneComponent.K2_GetComponentLocation` (`self.Sphere`))))

(event `ServerFireballHit`
  (params (actor_hit :type "Actor Object Reference") (location :type "Vector Structure"))
  (bind _damage (`self.damage`))
  (cast `/Game/Blueprints/Dragon/BP_RunnableDragon` actor_hit
    (:`CastFailed`
      (cast `/Game/Blueprints/Dragon/BP_Fireball` actor_hit
        (:`CastFailed`
          (`|ExecutionSequence`
            (:`then_0`
              ;[1 1 1] Deal Damage
              (if (`KismetSystemLibrary.DoesImplementInterface` actor_hit "/Game/Blueprints/Interfaces/BPI_Damageable.BPI_Damageable_C")
                (`GameplayStatics.ApplyDamage` actor_hit _damage null self)
                (`GameplayStatics.ApplyRadialDamage` _damage (`self.K2_GetActorLocation` self) 1000.0 null (`|MakeArray` actor_hit self :!type "Actor Object Reference") self)))
            (:`then_1`
              (`self.MulticastFireballExplosion` location))))))))

(event `MulticastFireballExplosion`
  (params (location :type "Vector Structure"))
  ;[1 1 1] Multicast Explosion And Sound
  (`GameplayStatics.SpawnEmitterAtLocation` "/Game/Assets/Particles/P_Explosion_FireBall.P_Explosion_FireBall" location)
  (`GameplayStatics.PlaySoundAtLocation` "/Game/StarterContent/Audio/Explosion01.Explosion01" location (struct) 1.0)
  (`self.K2_DestroyActor`)
  (`|SpawnActorFromClass` "/Game/Blueprints/Dragon/BP_Firebreath.BP_Firebreath_C" (`KismetMathLibrary.MakeTransform` (+ location (`KismetMathLibrary.RandomUnitVector`))) "Undefined" "OverrideRootScale"))

(event `self.ReceiveHit`
  (params (MyComp :type "PrimitiveComponent Object Reference") (Other :type "Actor Object Reference") (OtherComp :type "PrimitiveComponent Object Reference") (bSelfMoved :type Boolean) (HitLocation :type "Vector Structure") (HitNormal :type "Vector Structure") (NormalImpulse :type "Vector Structure") (Hit :type "HitResult Structure (by ref)"))
  (`self.ServerFireballHit` Other HitLocation))

(fn `UserConstructionScript`)