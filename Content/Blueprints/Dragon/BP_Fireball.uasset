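; BP_Fireball is a projectile actor that damages what it strikes and explodes.
; The construction script sets the projectile movement velocity from InitialVel.
; Overlap and hit events both feed ServerFireballHit, which ignores BP_RunnableDragon and other fireballs.
; For anything else, it sends faction-tagged damage through BPI_Damageable where implemented, then destroys itself and plays explosion particles and sound.
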(event `EventNewBullet`
  (set `MovementComponent.Velocity` (`self.InitialVel`) (`self.ProjectileMovement`)))

(event `self.ReceiveBeginPlay`)

(event `self.ReceiveTick`
  (params (DeltaSeconds :type "Float (single-precision)")))

(event `self.ReceiveActorBeginOverlap`
  (params (OtherActor :type "Actor Object Reference"))
  (`self.ServerFireballHit` OtherActor (`SceneComponent.K2_GetComponentLocation` (`self.Sphere`))))

(event `self.ReceiveHit`
  (params (MyComp :type "PrimitiveComponent Object Reference") (Other :type "Actor Object Reference") (OtherComp :type "PrimitiveComponent Object Reference") (bSelfMoved :type Boolean) (HitLocation :type "Vector Structure") (HitNormal :type "Vector Structure") (NormalImpulse :type "Vector Structure") (Hit :type "HitResult Structure (by ref)"))
  (`self.ServerFireballHit` Other HitLocation))

(event `ServerFireballHit`
  (params (actor_hit :type "Actor Object Reference") (location :type "Vector Structure"))
  (cast `/Game/Blueprints/Dragon/BP_RunnableDragon` actor_hit
    (:`CastFailed`
      (cast `/Game/Blueprints/Dragon/BP_Fireball` actor_hit
        (:`CastFailed`
          (`|ExecutionSequence`
            (:`then_0`
              ;[1 1 1] Deal Damage
              (if (`KismetSystemLibrary.DoesImplementInterface` actor_hit "/Game/Blueprints/Interfaces/BPI_Damageable.BPI_Damageable_C")
                (message `/Game/Blueprints/Interfaces/BPI_Damageable.ReceiveDamage` actor_hit (`self.damage`) self (`self.faction`))))
            (:`then_1`
              (`self.K2_DestroyActor`)
              (`GameplayStatics.SpawnEmitterAtLocation` "/Game/StarterContent/Particles/P_Explosion2.P_Explosion2" location)
              (`GameplayStatics.PlaySoundAtLocation` "/Game/StarterContent/Audio/Explosion01.Explosion01" location (struct) 1.0))))))))

(fn `UserConstructionScript`
  (`self.EventNewBullet`))