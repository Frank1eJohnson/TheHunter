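; BP_Firebreath is a fire breath projectile actor, launched at a preset velocity applied from the construction script.
; Overlaps and hits both route to ServerFirebreathHit, which ignores BP_RunnableDragon and BP_Fireball actors.
; Any other contact sends faction-tagged damage to targets implementing BPI_Damageable, then destroys the projectile with an explosion effect and sound.
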(event `self.ReceiveBeginPlay`)

(event `EventNewBreath`
  (set `MovementComponent.Velocity` (`self.ini_velocity_firebreath`) (`self.ProjectileMovement`)))

(event `self.ReceiveActorBeginOverlap`
  (params (OtherActor :type "Actor Object Reference")))

(event `self.ReceiveTick`
  (params (DeltaSeconds :type "Float (single-precision)")))

(event `self.ReceiveActorBeginOverlap`
  (params (OtherActor :type "Actor Object Reference"))
  (`self.ServerFirebreathHit` OtherActor (`SceneComponent.K2_GetComponentLocation` (`self.Sphere1`))))

(event `self.ReceiveHit`
  (params (MyComp :type "PrimitiveComponent Object Reference") (Other :type "Actor Object Reference") (OtherComp :type "PrimitiveComponent Object Reference") (bSelfMoved :type Boolean) (HitLocation :type "Vector Structure") (HitNormal :type "Vector Structure") (NormalImpulse :type "Vector Structure") (Hit :type "HitResult Structure (by ref)"))
  (`self.ServerFirebreathHit` Other HitLocation))

(event `ServerFirebreathHit`
  (params (actor_hit :type "Actor Object Reference") (location :type "Vector Structure"))
  (cast `/Game/Blueprints/Dragon/BP_RunnableDragon` actor_hit
    (:`CastFailed`
      (cast `/Game/Blueprints/Dragon/BP_Fireball` actor_hit
        (:`CastFailed`
          (`|ExecutionSequence`
            (:`then_0`
              ;[1 1 1] Deal Damage
              (if (`KismetSystemLibrary.DoesImplementInterface` actor_hit "/Game/Blueprints/Interfaces/BPI_Damageable.BPI_Damageable_C")
                (message `/Game/Blueprints/Interfaces/BPI_Damageable.ReceiveDamage` actor_hit (`self.damage_firebreath`) self (`self.faction_firebreath`))))
            (:`then_1`
              (`self.K2_DestroyActor`)
              (`GameplayStatics.SpawnEmitterAtLocation` "/Game/Assets/Particles/P_Explosion2.P_Explosion2" location)
              (`GameplayStatics.PlaySoundAtLocation` "/Game/StarterContent/Audio/Explosion01.Explosion01" location (struct) 1.0))))))))

(fn `UserConstructionScript`
  (`self.EventNewBreath`))