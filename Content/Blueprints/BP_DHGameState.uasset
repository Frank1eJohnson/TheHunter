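; BP_DHGameState is a game state Blueprint that tracks match start, match end and the winner in a dragon-versus-castle game.
; StartGame sets GameStarted, and the dragon death and castle destruction events each set a different Winner value and flag GameEnded.
; A GameEnded check makes the first of those outcomes final.
; The OnRep function for game start is empty, as are BeginPlay and Tick.
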(event `self.ReceiveBeginPlay`)

(event `self.ReceiveTick`
  (params (DeltaSeconds :type "Float (single-precision)")))

(event `OnDragonDead`
  (if (not (`self.game_ended`))
    (set `self.winner` "NewEnumerator1")
    (set `self.game_ended` true)))

(event `OnCastleDestroyed`
  (if (not (`self.game_ended`))
    (set `self.winner` "NewEnumerator0")
    (set `self.game_ended` true)))

(event `StartGame`
  (set `self.game_started` true))

(fn `OnRep_game_started`)

(fn `UserConstructionScript`)