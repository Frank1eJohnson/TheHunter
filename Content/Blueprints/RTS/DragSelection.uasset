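; RTS HUD that draws a drag-selection box and selects BP_RTSTestCharacter units inside it.
; While IsDrawing is set, DrawHUD stretches a texture from ClickedLocation to the mouse.
; Every such frame, units whose projected screen position passes IsInSelectionBox are appended to the first BP_RTSCam's Charactor array and get Selected called.
; The bounds test assumes a down-right drag, and repeated frames append without a duplicate check.
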(event `self.ReceiveBeginPlay`)

(event `self.ReceiveActorBeginOverlap`
  (params (OtherActor :type "Actor Object Reference")))

(event `self.ReceiveDrawHUD`
  (params (SizeX :type Integer) (SizeY :type Integer))
  (bind (_locationx _locationy) (`PlayerController.GetMousePosition` (`GameplayStatics.GetPlayerController` 0)))
  (bind (_x _y) (`KismetMathLibrary.BreakVector2D` (`self.ClickedLocation`)))
  (bind (_x_2 _y_2) (`KismetMathLibrary.BreakVector2D` (- (`self.CurrentMouseLocation`) (`self.ClickedLocation`))))
  (set `self.ScreenResolution` (`KismetMathLibrary.MakeVector2D` (`KismetMathLibrary.Conv_IntToDouble` SizeX) (`KismetMathLibrary.Conv_IntToDouble` SizeY)))
  (if (`self.IsDrawing`)
    (set `self.CurrentMouseLocation` (`KismetMathLibrary.MakeVector2D` _locationx _locationy))
    (`self.DrawTexture` "/Game/StarterContent/Textures/T_Metal_Copper_D.T_Metal_Copper_D" _x _y _x_2 _y_2)
    (bind _outactors (`GameplayStatics.GetAllActorsOfClass` "/Game/Blueprints/Soldiers/BP_RTSTestCharacter.BP_RTSTestCharacter_C"))
    (for _array_element _outactors
      (bind _result (`self.isInSelectionBox` _array_element _x _y _x_2 _y_2))
      (if _result
        (`KismetSystemLibrary.PrintString` "selected")
        (bind _outactors_2 (`GameplayStatics.GetAllActorsOfClass` "/Game/Blueprints/RTS/BP_RTSCam.BP_RTSCam_C"))
        (bind _charactor (`/Game/Blueprints/RTS/BP_RTSCam.Charactor` (`KismetArrayLibrary.Array_Get` _outactors_2)))
        (`KismetArrayLibrary.Array_Add` _charactor _array_element)
        (`KismetSystemLibrary.PrintString` (`KismetStringLibrary.Conv_IntToString` (`KismetArrayLibrary.Array_Length` _charactor)))
        (`/Game/Blueprints/Soldiers/BP_RTSTestCharacter.Selected` _array_element)))))

(event `self.ReceiveTick`
  (params (DeltaSeconds :type "Float (single-precision)")))

(fn `isInSelectionBox`
  (params (character :type "/Game/Blueprints/Soldiers/BP_RTSTestCharacter Object Reference") (X :type "Float (double-precision)") (Y :type "Float (double-precision)") (W :type "Float (double-precision)") (H :type "Float (double-precision)"))
  (returns (RESULT :type Boolean))
  (bind (_x _y) (`KismetMathLibrary.BreakVector2D` (`GameplayStatics.ProjectWorldToScreen` (`GameplayStatics.GetPlayerController` 0) (`self.K2_GetActorLocation` character))))
  (if (and (> _x X) (> _y Y) (< _x (+ X W)) (< _y (+ Y H)))
    (return true)
    (else
      (return false))))

(fn `UserConstructionScript`)