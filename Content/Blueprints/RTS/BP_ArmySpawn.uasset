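; BP_ArmySpawn is an RTS spawner that periodically creates army units on the server until it reaches MaxArmies.
; An authority-only looping timer from BeginPlay calls ServerSpawnArmy, which spawns BP_RTSTestCharacter with the first found BP_Castle's Level.
; Spawns fan out on alternating sides of the mesh along world Y, facing opposite the Sphere's yaw.
; IsArcher changes only the debug message, as both branches spawn the same class.
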(event `self.ReceiveBeginPlay`
  ;[1 1 1] spawn army
  (`/Engine/EditorBlueprintResources/ActorMacros.Switch Has Authority`
    (:`Authority`
      (`KismetSystemLibrary.K2_SetTimerDelegate` (delegate `EventSpawn`) (`self.Timer`) true))))

(event `ServerSpawnArmy`
  (bind _returnvalue (< (`self.num_of_armies`) (`self.max_armies`)))
  (bind (_returnvalue_x _returnvalue_y _returnvalue_z) (`KismetMathLibrary.BreakVector` (`SceneComponent.K2_GetComponentLocation` (`self.StaticMesh`))))
  (bind _returnvalue_2 (`KismetMathLibrary.MakeTransform` (`KismetMathLibrary.MakeVector` _returnvalue_x (+ _returnvalue_y (`self.LocationOffset`)) _returnvalue_z) (`KismetMathLibrary.MakeRotator` (.roll (.rotation (`SceneComponent.K2_GetComponentToWorld` (`self.Sphere`)))) (.pitch (.rotation (`SceneComponent.K2_GetComponentToWorld` (`self.Sphere`)))) (+ (.yaw (.rotation (`SceneComponent.K2_GetComponentToWorld` (`self.Sphere`)))) 180.0)) (.scale (`SceneComponent.K2_GetComponentToWorld` (`self.Sphere`)))))
  ;[1 1 1] spawn army
  (if (`self.IsArcher`)
    (if _returnvalue
      (bind _returnvalue_3 (`|SpawnActorFromClass` "/Game/Blueprints/Soldiers/BP_RTSTestCharacter.BP_RTSTestCharacter_C" _returnvalue_2 "AdjustIfPossibleButAlwaysSpawn" "OverrideRootScale"))
      ;;[1 1 1] Set Level
      (bind _outactors (`GameplayStatics.GetAllActorsOfClass` "/Game/Blueprints/Castle/BP_Castle.BP_Castle_C"))
      (set `/Game/Blueprints/Soldiers/BP_RTSTestCharacter.Level` (`/Game/Blueprints/Castle/BP_Castle.Level` (`KismetArrayLibrary.Array_Get` _outactors)) _returnvalue_3)
      (`KismetSystemLibrary.PrintString` "archer spawned")
      (set `self.num_of_armies` (+ (`self.num_of_armies`) 1) :!label _label)
      (if (< (`self.LocationOffset`) (* 10 (`self.LocationOffsetStep`)))
        (set `self.LocationOffset` (* (+ (`KismetMathLibrary.Abs` (`self.LocationOffset`)) (`self.LocationOffsetStep`)) (`self.Flag`)))
        (else
          (set `self.LocationOffset` 0.0)))
      (set `self.Flag` (* (`self.Flag`) -1.0)))
    (elif _returnvalue
      (bind _returnvalue_4 (`|SpawnActorFromClass` "/Game/Blueprints/Soldiers/BP_RTSTestCharacter.BP_RTSTestCharacter_C" _returnvalue_2 "AdjustIfPossibleButAlwaysSpawn" "OverrideRootScale"))
      (bind _outactors_2 (`GameplayStatics.GetAllActorsOfClass` "/Game/Blueprints/Castle/BP_Castle.BP_Castle_C"))
      (set `/Game/Blueprints/Soldiers/BP_RTSTestCharacter.Level` (`/Game/Blueprints/Castle/BP_Castle.Level` (`KismetArrayLibrary.Array_Get` _outactors_2)) _returnvalue_4)
      (`KismetSystemLibrary.PrintString` "swordsman spawned")
      (goto _label))))

(event `EventSpawn`
  ;[1 1 1] spawn army
  (`self.ServerSpawnArmy`))

(fn `UserConstructionScript`)