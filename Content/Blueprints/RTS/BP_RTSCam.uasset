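; RTS camera that pans, rotates and lets the player select characters and order them to move.
; Axis input, screen edges and gated middle-mouse drag (Shift to pan) drive it, with a downward trace setting height after axis moves.
; ToggleFlyingMode jumps to the first BP_Castle found at construction.
; A looping timer feeds the transform to ServerSyncLocation, while right-click orders for selected BPI_RTSMovable characters go through ServerMoveCharacterTo.
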(event `InputAxisKey|MouseX`
  (params (AxisValue :type "Float (single-precision)"))
  ;[1 1 1] Camera Translate & Rotate
  (`/Engine/EditorBlueprintResources/StandardMacros.Gate` true :!label _label
    (:`Exit`
      (`self.K2_AddActorLocalOffset` (`KismetMathLibrary.MakeVector` 0.0 (* -1 (* (`self.panningSpeed`) AxisValue)))))))

(event `Key|LeftShift`
  (params (Key :type "Key Structure" :default "AnyKey"))
  ;[1 1 1] Camera Translate & Rotate
  (:`Pressed`
    (set `self.TPanFRotate` true))
  (:`Released`
    (set `self.TPanFRotate` false)))

(event `self.ReceiveTick`
  (params (DeltaSeconds :type "Float (single-precision)")))

(event `InputAxisKey|MouseY`
  (params (AxisValue :type "Float (single-precision)"))
  ;[1 1 1] Camera Translate & Rotate
  (`/Engine/EditorBlueprintResources/StandardMacros.Gate` true :!label _label_2
    (:`Exit`
      (`self.K2_AddActorLocalOffset` (`KismetMathLibrary.MakeVector` (* -1 (* (`self.panningSpeed`) AxisValue)))))))

(event `self.ReceiveActorBeginOverlap`
  (params (OtherActor :type "Actor Object Reference")))

(event `InputAction|ToggleFlyingMode`
  (params (Key :type "Key Structure" :default "AnyKey"))
  (bind _castle (`self.castle`))
  (:`Pressed`
    (`/Engine/EditorBlueprintResources/StandardMacros.IsValid` _castle
      (:`Is Valid`
        (`self.K2_SetActorLocation` (`SceneComponent.K2_GetComponentLocation` (`/Game/Blueprints/Castle/BP_Castle.Capsule` _castle)))))))

(event `InputAxisKey|MouseX`
  (params (AxisValue :type "Float (single-precision)"))
  (bind _returnvalue (* (`GameplayStatics.GetWorldDeltaSeconds`) (`self.ScreenEdgeMoveSpeed`)))
  (bind _returnvalue_2 (/ (`PlayerController.GetMousePosition` (`GameplayStatics.GetPlayerController` 0)) (`KismetMathLibrary.BreakVector2D` (`WidgetLayoutLibrary.GetViewportSize`))))
  ;[1 1 1] screenedgemove
  (`|ExecutionSequence`
    (:`then_0`
      (if (> _returnvalue_2 0.98)
        (`self.K2_AddActorLocalOffset` (`KismetMathLibrary.MakeVector` 0.0 _returnvalue) true)))
    (:`then_1`
      (if (< _returnvalue_2 0.02)
        (`self.K2_AddActorLocalOffset` (`KismetMathLibrary.MakeVector` 0.0 (* -1 _returnvalue)) true)))))

(event `self.ReceiveBeginPlay`
  ;[1 1 1] Sync Location And Rotation
  (`KismetSystemLibrary.K2_SetTimerDelegate` (delegate `SyncLocation`) 0.5 true))

(event `Key|MiddleMouseButton`
  (params (Key :type "Key Structure" :default "AnyKey"))
  (bind _returnvalue (`GameplayStatics.GetPlayerController` 0))
  (bind (_returnvalue_roll _returnvalue_pitch _returnvalue_yaw) (`KismetMathLibrary.BreakRotator` (`SceneComponent.K2_GetComponentRotation` (`self.Camera`))))
  ;[1 1 1] Camera Translate & Rotate
  (:`Pressed`
    (if (`self.TPanFRotate`)
      (set `PlayerController.bShowMouseCursor` false _returnvalue)
      (`|ExecutionSequence`
        (:`then_0`
          (goto _label :!via `Open`))
        (:`then_1`
          (goto _label_2 :!via `Open`)))
      (else
        (set `PlayerController.bShowMouseCursor` false _returnvalue)
        (`|ExecutionSequence`
          (:`then_0`
            (goto _label_3 :!via `Open`))
          (:`then_1`
            (goto _label_4 :!via `Open`))))))
  (:`Released`
    ;;[1 1 1] close gate
    (set `PlayerController.bShowMouseCursor` true _returnvalue)
    (`|ExecutionSequence`
      (:`then_0`
        (goto _label_3 :!via `Close`))
      (:`then_1`
        (goto _label_4 :!via `Close`))
      (:`then_2`
        (goto _label :!via `Close`))
      (:`then_3`
        (goto _label_2 :!via `Close`)))))

(event `SyncLocation`
  ;[1 1 1] Sync Location And Rotation
  (`self.ServerSyncLocation` (`self.K2_GetActorLocation`) (`self.K2_GetActorRotation`)))

(event `InputAxis|MoveForward`
  (params (AxisValue :type "Float (single-precision)"))
  (`self.K2_AddActorLocalOffset` (`KismetMathLibrary.MakeVector` (* AxisValue (`self.moveSpeed`))))
  (`self.SlopeDetection`))

(event `ServerSyncLocation`
  (params (location :type "Vector Structure") (rotation :type "Rotator Structure"))
  ;[1 1 1] Sync Location And Rotation
  (`self.K2_SetActorLocationAndRotation` location rotation true))

(event `InputAxisKey|MouseX`
  (params (AxisValue :type "Float (single-precision)"))
  ;[1 1 1] Camera Translate & Rotate
  (`/Engine/EditorBlueprintResources/StandardMacros.Gate` true :!label _label_3
    (:`Exit`
      (`self.K2_AddActorLocalRotation` (`KismetMathLibrary.MakeRotator` 0.0 0.0 (* (`self.rotateSpeed`) AxisValue))))))

(event `Key|H`
  (params (Key :type "Key Structure" :default "AnyKey"))
  (:`Pressed`
    (`KismetSystemLibrary.PrintString` "Hello")))

(event `InputAxis|MoveRight`
  (params (AxisValue :type "Float (single-precision)"))
  (`self.K2_AddActorLocalOffset` (`KismetMathLibrary.MakeVector` 0.0 (* AxisValue (`self.moveSpeed`))))
  (`self.SlopeDetection`))

(event `InputAxisKey|MouseY`
  (params (AxisValue :type "Float (single-precision)"))
  (bind _returnvalue (* (`GameplayStatics.GetWorldDeltaSeconds`) (`self.ScreenEdgeMoveSpeed`)))
  (bind _returnvalue_2 (/ (`.LocationY` (`PlayerController.GetMousePosition` (`GameplayStatics.GetPlayerController` 0))) (`.Y` (`KismetMathLibrary.BreakVector2D` (`WidgetLayoutLibrary.GetViewportSize`)))))
  ;[1 1 1] screenedgemove
  (`|ExecutionSequence`
    (:`then_0`
      (if (> _returnvalue_2 0.98)
        (`self.K2_AddActorLocalOffset` (`KismetMathLibrary.MakeVector` _returnvalue) true)))
    (:`then_1`
      (if (< _returnvalue_2 0.02)
        (`self.K2_AddActorLocalOffset` (`KismetMathLibrary.MakeVector` _returnvalue) true)))))

(event `InputAxisKey|MouseY`
  (params (AxisValue :type "Float (single-precision)"))
  (bind (_returnvalue_roll _returnvalue_pitch _returnvalue_yaw) (`KismetMathLibrary.BreakRotator` (`SceneComponent.K2_GetComponentRotation` (`self.Camera`))))
  ;[1 1 1] Camera Translate & Rotate
  (`/Engine/EditorBlueprintResources/StandardMacros.Gate` true :!label _label_4
    (:`Exit`
      (`SceneComponent.K2_SetWorldRotation` (`self.Camera`) (`KismetMathLibrary.MakeRotator` _returnvalue_roll (`KismetMathLibrary.FClamp` (+ (* (`self.rotateSpeed`) AxisValue) _returnvalue_pitch) -89.0 -1.0) _returnvalue_yaw) false false))))

(event `Key|LeftMouseButton`
  (params (Key :type "Key Structure" :default "AnyKey"))
  ;[1 1 1] lock viewport
  (:`Released`
    (bind _asunused_rtsplayer_controller (cast `/Game/Blueprints/UNUSED_RTSPlayerController` (`GameplayStatics.GetPlayerController` 0)))
    (`/Game/Blueprints/UNUSED_RTSPlayerController.LockMouseToViewPort` _asunused_rtsplayer_controller)))

(event `Key|RightMouseButton`
  (params (Key :type "Key Structure" :default "AnyKey"))
  ;[1 1 1] lock viewport
  (:`Released`
    (bind _asunused_rtsplayer_controller (cast `/Game/Blueprints/UNUSED_RTSPlayerController` (`GameplayStatics.GetPlayerController` 0)))
    (`/Game/Blueprints/UNUSED_RTSPlayerController.LockMouseToViewPort` _asunused_rtsplayer_controller)))

(event `SlopeDetection`
  (bind (_returnvalue_x _returnvalue_y) (`KismetMathLibrary.BreakVector` (`self.K2_GetActorLocation`)))
  (bind _returnvalue (`SceneComponent.K2_GetComponentLocation` (`self.Camera`)))
  ;[1 1 1] SlopeDetection
  (bind _outhit (`KismetSystemLibrary.LineTraceSingle` _returnvalue (+ _returnvalue (0.0 0.0 -10000.0)) "TraceTypeQuery1"))
  (`self.K2_SetActorLocation` (`KismetMathLibrary.MakeVector` _returnvalue_x _returnvalue_y (.z (`.Location` (`GameplayStatics.BreakHitResult` _outhit))))))

(event `Key|LeftMouseButton`
  (params (Key :type "Key Structure" :default "AnyKey"))
  (bind (_bblockinghit _binitialoverlap _time _location _impactpoint _normal _impactnormal _physmat _hitactor _hitcomponent) (`GameplayStatics.BreakHitResult` (`PlayerController.GetHitResultUnderCursorByChannel` (`GameplayStatics.GetPlayerController` 0) "TraceTypeQuery2" true)))
  ;[1 1 1] Select and move character
  (:`Pressed`
    (bind _ascharacter (cast `Character` _hitactor)
      (:`then`
        (if (`KismetSystemLibrary.DoesImplementInterface` _ascharacter "/Game/Blueprints/Interfaces/BPI_RTSMovable.BPI_RTSMovable_C")
          (`KismetSystemLibrary.PrintString` "Yes my lord!")
          (bind _asbp_rtstest_character (cast `/Game/Blueprints/Soldiers/BP_RTSTestCharacter` _ascharacter)
            (:`then`
              (`SceneComponent.SetVisibility` (`self.Decal`) false false)
              (bind _output_get (set `self.Decal` (`/Game/Blueprints/Soldiers/BP_RTSTestCharacter.Decal` _asbp_rtstest_character)))
              (`SceneComponent.SetVisibility` _output_get true false)
              (goto _label_5 :!via `Open`))
            (:`CastFailed`
              (goto _label_5 :!via `Open`)))
          (else
            (goto _label_5 :!via `Close`))))
      (:`CastFailed`
        (`SceneComponent.SetVisibility` (`self.Decal`) false false)
        (goto _label_5 :!via `Close`)))))

(event `ServerMoveCharacterTo`
  (params (movingChar :type "Character Object Reference") (destination :type "Vector Structure"))
  ;[1 1 1] Select and move character
  (message `/Game/Blueprints/Interfaces/BPI_RTSMovable.Move Character To` movingChar destination))

(event `Key|RightMouseButton`
  (params (Key :type "Key Structure" :default "AnyKey"))
  ;[1 1 1] Select and move character
  (:`Pressed`
    (`/Engine/EditorBlueprintResources/StandardMacros.Gate` true :!label _label_5
      (:`Exit`
        (`KismetSystemLibrary.PrintString` "On my way!")
        (`self.ServerMoveCharacterTo` (stale `Key|LeftMouseButton` _ascharacter) (`.Location` (`GameplayStatics.BreakHitResult` (`PlayerController.GetHitResultUnderCursorByChannel` (`GameplayStatics.GetPlayerController` 0) "TraceTypeQuery2" true))))))))

(fn `UserConstructionScript`
  (bind _outactors (`GameplayStatics.GetAllActorsOfClass` "/Game/Blueprints/Castle/BP_Castle.BP_Castle_C"))
  (if (> (`KismetArrayLibrary.Array_Length` _outactors) 0)
    (bind _asbp_castle (cast `/Game/Blueprints/Castle/BP_Castle` (`KismetArrayLibrary.Array_Get` _outactors)))
    (set `self.castle` _asbp_castle)))