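; BP_DragonNest is a nest actor meant to heal dragons that are near it.
; On the server each Tick, it acts on overlapping BP_RunnableDragon actors only while no BP_RTSTestCharacter overlaps the nest.
; Healing goes through ApplyDamage, passing HealPerSecond scaled by delta time unnegated, so the effect depends on that value's sign and the dragon's damage handling.
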(event `self.ReceiveBeginPlay`)

(event `self.ReceiveActorBeginOverlap`
  (params (OtherActor :type "Actor Object Reference")))

(event `self.ReceiveTick`
  (params (DeltaSeconds :type "Float (single-precision)"))
  ;[1 1 1] Heal the Dragon When Near
  (`/Engine/EditorBlueprintResources/ActorMacros.Switch Has Authority`
    (:`Authority`
      (if (<= (`KismetArrayLibrary.Array_Length` (`self.GetOverlappingActors` "/Game/Blueprints/Soldiers/BP_RTSTestCharacter.BP_RTSTestCharacter_C")) 0)
        (for _array_element (`self.GetOverlappingActors` "/Game/Blueprints/Dragon/BP_RunnableDragon.BP_RunnableDragon_C")
          (bind _asbp_runnable_dragon (cast `/Game/Blueprints/Dragon/BP_RunnableDragon` _array_element))
          (`/Engine/EditorBlueprintResources/StandardMacros.IsValid` _asbp_runnable_dragon
            (:`Is Valid`
              (`GameplayStatics.ApplyDamage` _asbp_runnable_dragon (* (`self.heal_per_second`) DeltaSeconds)))))))))

(fn `UserConstructionScript`)