(event Custom|MC_RefreshHealthBar
  ;[1 1 1] Receive damage
  (CallFunction|RefreshHealthBar))

(event Custom|ServerShootArrow
  (params (target_actor :type Actor%20Object%20Reference))
  ;[1 1 1] Attack
  (for _array_element (Components|GetChildrenComponents (Variables|Components|GetRow1) false)
    (CallFunction|ShootSingleArrow target_actor (Transformation|GetWorldLocation _array_element)))
  (Development|PrintString "arrows shot"))

(event Custom|ServerMoveCharacter
  (params (location :type Vector))
  ;[1 1 1] Move
  (bind _asrtsaicontroller (Utilities|Casting|CastToRTSAIController (Pawn|GetController)))
  (Class|BPIRTSMovable|MoveCharacterto(Message) _asrtsaicontroller location))

(event EventTick
  (params (DeltaSeconds :type Float%20%28single-precision%29))
  ;[1 1 1] Attack
  (Networking|SwitchHasAuthority
    (:Authority
      (Utilities|FlowControl|Sequence
        (:then_0
          (if (> (Variables|Default|Getattacking_cooldown_remain) 0.0)
            (Variables|Default|Setattacking_cooldown_remain (- (Variables|Default|Getattacking_cooldown_remain) DeltaSeconds))))
        (:then_1
          (if (<= (Variables|Default|Getattacking_cooldown_remain) 0.0)
            (bind _outactors (Actor|GetAllActorsOfClass "/Game/Blueprints/Dragon/BP_RunnableDragon.BP_RunnableDragon_C"))
            (if (> (Utilities|Array|Length _outactors) 0)
              (if (< (Math|Vector|VectorLength (- (Transformation|GetActorLocation (Utilities|Array|Get(acopy) _outactors)) (+ (* (Math|Vector|GetForwardVector (Transformation|GetActorRotation)) 3e+01) (+ (Transformation|GetActorLocation) "0, 0,40.000000")))) (Variables|Default|Getmax_attack_range))
                (if (not (> (Math|Vector|VectorLength (Transformation|GetVelocity)) 0.0))
                  (Variables|Default|Setattacking_cooldown_remain (+ (Variables|Default|Getattacking_cooldown_remain) (Variables|Default|Getattacking_cooldown)))
                  (CallFunction|ServerShootArrow (Utilities|Array|Get(acopy) _outactors)))))))))))

(event EventMoveCharacterto
  (params (Location :type Vector))
  ;[1 1 1] Move
  (CallFunction|ServerMoveCharacter Location))

(event Game|Damage|EventAnyDamage
  (params (Damage :type Float%20%28single-precision%29) (DamageType :type Damage%20Type%20Object%20Reference) (InstigatedBy :type Controller%20Object%20Reference) (DamageCauser :type Actor%20Object%20Reference))
  ;[1 1 1] Receive damage
  (Health|UpdateHealth Damage)
  (CallFunction|MCRefreshHealthBar))

(fn ConstructionScript
  (bind _returnvalue (Rendering|Material|CreateDynamicMaterialInstance (Variables|Default|Gethealth_bar) 0 "/Game/Assets/Materials/M_HealthBar.M_HealthBar" :!class /Script/Engine.PrimitiveComponent))
  (Variables|Default|Sethealth_material _returnvalue)
  (CallFunction|RefreshHealthBar))

(fn CaculateArrowAction
  (params (Target :type Vector) (Origin :type Vector) (Speed :type Float%20%28single-precision%29) (Gravity :type Float%20%28single-precision%29))
  (bind _returnvalue (- Target Origin))
  (bind _returnvalue_2 (Math|Float|Square Speed))
  (bind _returnvalue_3 (Math|Float|Square (.x _returnvalue)))
  (bind _returnvalue_4 (Math|Float|Square (.y _returnvalue)))
  (bind _returnvalue_5 (* _returnvalue_2 2.0))
  (bind _returnvalue_6 (+ _returnvalue_3 _returnvalue_4))
  (bind _returnvalue_7 (Math|Float|Sqrt _returnvalue_6))
  (bind _returnvalue_8 (/ (.z _returnvalue) _returnvalue_7))
  (bind _returnvalue_9 (* Gravity _returnvalue_7))
  (bind _returnvalue_10 (/ _returnvalue_9 _returnvalue_5))
  (bind _returnvalue_11 (- _returnvalue_10 _returnvalue_8))
  (bind _returnvalue_12 (* _returnvalue_10 2.0))
  (bind _returnvalue_13 (* _returnvalue_11 _returnvalue_10))
  (bind _returnvalue_14 (* _returnvalue_13 4.0))
  (bind _returnvalue_15 (- 1.0 _returnvalue_14))
  (bind _returnvalue_16 (Math|Float|Sqrt _returnvalue_15))
  (bind _returnvalue_17 (+ -1.0 _returnvalue_16))
  (bind _returnvalue_18 (/ _returnvalue_17 _returnvalue_12))
  (if (== _returnvalue_18 0.0)
    (Development|PrintString "no resaults" true true "(R=1.000000,G=0.977679,B=0.120170,A=1.000000)" 1e+01)
    (return "0.000000,0,0")
    (else
      (return (Math|Vector|Normalize (Math|Vector|MakeVector (.x _returnvalue) (.y _returnvalue) (* _returnvalue_7 _returnvalue_18)))))))

(fn ShootSingleArrow
  (params (target :type Actor%20Object%20Reference) (shootFrom :type Vector))
  (bind (_ret_damage _ret_speed _ret_stamina_damage) (Attack|GetArrowDamageandSpeedbyLevel))
  (bind _direction (Attack|CaculateArrowAction (Transformation|GetActorLocation target) shootFrom _ret_speed -4.9e+02))
  (bind _returnvalue (Game|SpawnActorfromClass "/Game/Blueprints/Soldiers/BP_Arrow.BP_Arrow_C" (Math|Transform|MakeTransform shootFrom (Math|Conversions|RotationFromXVector (Class|DragonHuntHelperLibrary|RotateTowardsRandomDirection _direction (Math|Random|RandomFloatinRange 0.0 (Variables|Default|Getattacking_max_angle))))) "AlwaysSpawn" 0 0))
  (Utilities|IsValid _returnvalue
    (:Is%20Valid
      (Default|Initialize _returnvalue _ret_damage _ret_speed _ret_stamina_damage))))

(fn GetArrowDamageandSpeedbyLevel
  (bind _arrow_damage (Variables|Default|Getarrow_damage))
  (bind _level (Variables|Default|GetLevel))
  (bind _arrow_speed (Variables|Default|Getarrow_speed))
  (bind _level_2 (Variables|Default|GetLevel))
  (bind _stamina_damage (Variables|Default|Getstamina_damage))
  (bind _level_3 (Variables|Default|GetLevel))
  (bind _returnvalue (Utilities|Array|Length _stamina_damage))
  (bind _returnvalue_2 (Utilities|Array|Length _arrow_speed))
  (bind _returnvalue_3 (Utilities|Array|Length _arrow_damage))
  (Utilities|FlowControl|Sequence
    (:then_0
      ;[1 1 1] Calculate Damage Based On Level
      (if (>= _level _returnvalue_3)
        (LocalVariables|Setcurrent_damage (Utilities|Array|Get(acopy) _arrow_damage (- _returnvalue_3 1)))
        (else
          (LocalVariables|Setcurrent_damage (Utilities|Array|Get(acopy) _arrow_damage _level)))))
    (:then_1
      ;[1 1 1] Calculate Speed Based On Level
      (if (>= _level_2 _returnvalue_2)
        (LocalVariables|Setcurrent_speed (Utilities|Array|Get(acopy) _arrow_speed (- _returnvalue_2 1)))
        (else
          (LocalVariables|Setcurrent_speed (Utilities|Array|Get(acopy) _arrow_speed _level_2)))))
    (:then_2
      ;[1 1 1] Calculate Stamina Dam Based On Level
      (if (>= _level_3 _returnvalue)
        (LocalVariables|Setcurrent_stamina_damage (Utilities|Array|Get(acopy) _stamina_damage (- _returnvalue 1)))
        (else
          (LocalVariables|Setcurrent_stamina_damage (Utilities|Array|Get(acopy) _stamina_damage _level_3)))))
    (:then_3
      ;[1 1 1] Return
      (return (LocalVariables|Getcurrent_damage) (LocalVariables|Getcurrent_speed) (LocalVariables|Getcurrent_stamina_damage)))))

(fn UNUSEDUpdateHealthBar)

(fn UpdateHealth
  (params (Damage%20Amount :type Float%20%28single-precision%29))
  (Variables|Health|Setcurrent_health (Math|Float|Clamp(Float) (- (Variables|Health|Getcurrent_health) Damage%20Amount) 0.0 (Variables|Health|Gettotal_health)))
  (if (<= (Variables|Health|Getcurrent_health) 0.0)
    (Actor|DestroyActor)))

(fn Selected)

(fn Deselected)

(fn RefreshHealthBar
  (Rendering|Material|SetScalarParameterValue (Variables|Default|Gethealth_material) "percentage" (Math|Float|Clamp(Float) (/ (Variables|Health|Getcurrent_health) (Variables|Health|Gettotal_health))) :!class /Script/Engine.MaterialInstanceDynamic))