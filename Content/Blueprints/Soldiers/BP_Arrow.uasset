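; BP_Arrow is a soldier's arrow projectile that hurts dragons on contact.
; Initialize stores damage, stamina damage and speed, then multicasts transform and local velocity to the ProjectileMovement component.
; Each tick it faces its velocity and counts down a lifetime before destroying itself.
; Only the server handles overlaps, applying health and stamina damage to BP_RunnableDragon and destroying the arrow, while other actors are unaffected.
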(event `self.ReceiveTick`
  (params (DeltaSeconds :type "Float (single-precision)"))
  (`self.SetActorRotation` (`KismetMathLibrary.Conv_VectorToRotator` (`self.GetVelocity`)))
  (bind _output_get (set `self.lifetime_remaining` (- (`self.lifetime_remaining`) DeltaSeconds)))
  (if (< _output_get 0.0)
    (`self.K2_DestroyActor`)))

(event `self.ReceiveActorBeginOverlap`
  (params (OtherActor :type "Actor Object Reference"))
  (`/Engine/EditorBlueprintResources/ActorMacros.Switch Has Authority`
    (:`Authority`
      (`self.ServerCollisionCheck` OtherActor))))

(event `self.ReceiveBeginPlay`)

(event `ServerCollisionCheck`
  (params (other :type "Actor Object Reference"))
  (if (`KismetMathLibrary.ClassIsChildOf` (`GameplayStatics.GetObjectClass` other) "/Game/Blueprints/Dragon/BP_RunnableDragon.BP_RunnableDragon_C")
    (bind _asbp_runnable_dragon (cast `/Game/Blueprints/Dragon/BP_RunnableDragon` other))
    (message `/Game/Blueprints/Interfaces/BPI_Damageable.ReceiveDamage` _asbp_runnable_dragon (`self.Damage`) null 0)
    (`/Game/Blueprints/Dragon/BP_RunnableDragon.Receive Stamina Damage` _asbp_runnable_dragon (`self.stamina_damage`) null 0)
    (`self.K2_DestroyActor`)
    (elif (`KismetMathLibrary.ClassIsChildOf` (`GameplayStatics.GetObjectClass` other) "/Game/Blueprints/Soldiers/BP_RTSTestCharacter.BP_RTSTestCharacter_C")
      _)))

(event `self.ReceiveActorBeginOverlap`
  (params (OtherActor :type "Actor Object Reference")))

(event `multicastVelocityAndTransform`
  (params (local_velocity :type "Vector Structure") (location :type "Vector Structure") (rotation :type "Rotator Structure"))
  (`self.K2_SetActorLocationAndRotation` location rotation)
  (`ProjectileMovementComponent.SetVelocityInLocalSpace` (`self.ProjectileMovement`) local_velocity))

(fn `Initialize`
  (params (Damage :type "Float (double-precision)") (Speed :type "Float (double-precision)") (stamina_damage :type "Float (double-precision)"))
  (set `self.Damage` Damage)
  (set `self.stamina_damage` stamina_damage)
  (bind _output_get (set `self.Speed` Speed))
  (`self.multicastVelocityAndTransform` (`KismetMathLibrary.MakeVector` _output_get) (.location (`self.GetTransform`)) (.rotation (`self.GetTransform`))))

(fn `UserConstructionScript`
  (set `self.lifetime_remaining` (`self.lifetime`)))