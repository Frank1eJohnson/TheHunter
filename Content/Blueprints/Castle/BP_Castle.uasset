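; Castle actor with a health pool shown on a text component and a gold-based level upgrade.
; AnyDamage lowers clamped health, destroys the actor when the check reaches zero, and refreshes the text.
; Upgrade spends gold to raise the level and the next cost, or prints a warning when gold is short.
; The construction script creates dynamic material instances for each mesh material and initializes the health text.
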(event `self.ReceiveBeginPlay`)

(event `self.ReceiveActorBeginOverlap`
  (params (OtherActor :type "Actor Object Reference")))

(event `self.ReceiveTick`
  (params (DeltaSeconds :type "Float (single-precision)")))

(event `self.ReceiveAnyDamage`
  (params (Damage :type "Float (single-precision)") (DamageType :type "DamageType Object Reference") (InstigatedBy :type "Controller Object Reference") (DamageCauser :type "Actor Object Reference"))
  (bind _returnvalue (`KismetMathLibrary.FClamp` (- (`self.current_health`) Damage) 0.0 (`self.max_health`)))
  (`|ExecutionSequence`
    (:`then_0`
      (set `self.current_health` _returnvalue)
      (if (<= _returnvalue 0.0)
        (`self.BeginToDie`)))
    (:`then_1`
      (`self.refreshText`))))

(event `/Game/Blueprints/Interfaces/BPI_Damageable.ReceiveDamage`
  (params (damage_amount :type "Float (single-precision)") (source :type "Actor Object Reference") (source_faction :type Integer)))

(event `/Game/Blueprints/Interfaces/BPI_Damageable.BeginToDie`
  (`self.K2_DestroyActor`))

(fn `getHealthString`
  (returns (health_string :type String))
  (return (`KismetStringLibrary.Concat_StrStr` (`KismetStringLibrary.Conv_DoubleToString` (`self.current_health`)) " / " (`KismetStringLibrary.Conv_DoubleToString` (`self.max_health`)))))

(fn `GetUpgradeString`
  (returns (NewParam :type String))
  (return (`KismetStringLibrary.Concat_StrStr` (`KismetStringLibrary.Conv_IntToString` (`self.TotalGold`)) "/" (`KismetStringLibrary.Conv_IntToString` (`self.GoldNeededforNextLevel`)))))

(fn `refreshText`
  (bind _health_string (`self.getHealthString`))
  (`TextRenderComponent.K2_SetText` (`self.HealthText_temp`) (`KismetTextLibrary.Conv_StringToText` _health_string)))

(fn `Upgrade`
  (bind _goldneededfornextlevel (`self.GoldNeededforNextLevel`))
  (bind _totalgold (`self.TotalGold`))
  (if (> _totalgold _goldneededfornextlevel)
    (set `self.TotalGold` (- _totalgold _goldneededfornextlevel))
    (set `self.Level` (+ (`self.Level`) 1))
    (set `self.GoldNeededforNextLevel` (+ (`self.GoldNeededforNextLevel`) (* (`self.Level`) 1000)))
    (else
      (`KismetSystemLibrary.PrintString` "you need to gain more gold!!!"))))

(fn `UserConstructionScript`
  (`|ExecutionSequence`
    (:`then_0`
      (for (_array_element _array_index) (`MeshComponent.GetMaterials` (`self.StaticMesh`))
        (`PrimitiveComponent.CreateDynamicMaterialInstance` (`self.StaticMesh`) _array_index _array_element)))
    (:`then_1`
      (`self.refreshText`))))