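; BP_Mine is a gold mine that fills a progress bar while RTS characters stand inside its sphere collision and drains it otherwise.
; Each Tick updates the clamped progress and pushes it to a dynamic material's "percentage" parameter.
; A full bar resets and adds gold to the first BP_Castle found, upgrading it past its gold threshold.
; Overlap-based army counting and timer nodes are left disconnected.
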(event Custom|reset_progress
  (Variables|Default|Setprogress 0.0))

(event Custom|AddGold
  (bind _outactors (Actor|GetAllActorsOfClass "/Game/Blueprints/Castle/BP_Castle.BP_Castle_C"))
  (if (> (Utilities|Array|Length _outactors) 0)
    (bind _output_get (Variables|/Game/Blueprints/Castle/BP_Castle.BP_Castle_C|SetTotalGold (Utilities|Array|Get(acopy) _outactors) (+ (Variables|/Game/Blueprints/Castle/BP_Castle.BP_Castle_C|GetTotalGold (Utilities|Array|Get(acopy) _outactors)) 300)))
    (if (> _output_get (Variables|/Game/Blueprints/Castle/BP_Castle.BP_Castle_C|GetGoldNeededforNextLevel (Utilities|Array|Get(acopy) _outactors)))
      (Default|Upgrade (Utilities|Array|Get(acopy) _outactors)))))

(event Collision|EventActorEndOverlap
  (params (OtherActor :type Actor%20Object%20Reference)))

(event EventTick
  (params (DeltaSeconds :type Float%20%28single-precision%29)))

(event Collision|EventActorBeginOverlap
  (params (OtherActor :type Actor%20Object%20Reference)))

(event EventTick
  (params (DeltaSeconds :type Float%20%28single-precision%29))
  (CallFunction|ProgressGold DeltaSeconds)
  (if (>= (Variables|Default|Getprogress) 1.0)
    (Utilities|FlowControl|Sequence
      (:then_0
        (CallFunction|ResetProgress))
      (:then_1
        (CallFunction|AddGold)))))

(fn ConstructionScript
  (bind _returnvalue (Rendering|Material|CreateDynamicMaterialInstance (Variables|Default|GetGoldProgressBar) 0 "/Game/Assets/Materials/M_GoldProgressBar.M_GoldProgressBar" :!class /Script/Engine.PrimitiveComponent))
  (Variables|Default|Setgold_progress_instance _returnvalue)
  (CallFunction|RefreshBar))

(fn ProgressGold
  (params (delta_time :type Float%20%28single-precision%29))
  (if (> (Utilities|Array|Length (Collision|GetOverlappingActors (Variables|Default|GetSphereCollision) "/Game/Blueprints/Soldiers/BP_RTSTestCharacter.BP_RTSTestCharacter_C" :!class /Script/Engine.PrimitiveComponent)) 0)
    (LocalVariables|Setdelta_progress (* (Variables|Default|Getprogress_per_second) delta_time))
    (else
      (LocalVariables|Setdelta_progress (* (Variables|Default|Getprogress_lose_per_second) -1.0 delta_time))))
  (Variables|Default|Setprogress (Math|Float|Clamp(Float) (+ (Variables|Default|Getprogress) (LocalVariables|Getdelta_progress))))
  (CallFunction|RefreshBar))

(fn RefreshBar
  (Rendering|Material|SetScalarParameterValue (Variables|Default|Getgold_progress_instance) "percentage" (Variables|Default|Getprogress) :!class /Script/Engine.MaterialInstanceDynamic))